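; BP_JadeWorkbench is the workbench for the jade betting game, displaying three tool components that track the current tool mode.
; OnToolModeChanged switches on the new mode: window cutter, flashlight or combined flashlight-cutter each hide one matching tool and show the other two.
; The no-tool mode shows all three, so the bench appears to hold whichever tools are not in use.
; Construction script, BeginPlay and Tick are empty.
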(event EventBeginPlay)

(event Collision|EventActorBeginOverlap
  (params (OtherActor :type Actor%20Object%20Reference)))

(event EventTick
  (params (DeltaSeconds :type Float%20%28single-precision%29)))

(event EventOnToolModeChanged
  (params (NewMode :type EClcToolMode%20Enum :default "Opener"))
  (switch Utilities|FlowControl|Switch|SwitchonEClcToolMode NewMode
    (:Opener
      (Rendering|SetVisibility (Variables|Default|GetTool_04) false false)
      (Rendering|SetVisibility (Variables|Default|GetTool_03) true false))
    (:Flashlight
      (Rendering|SetVisibility (Variables|Default|GetTool_04) true false)
      (Rendering|SetVisibility (Variables|Default|GetTool_03) false false))
    (:Combined
      (Rendering|SetVisibility (Variables|Default|GetTool_04) true false)
      (Rendering|SetVisibility (Variables|Default|GetTool_02) false false))
    (:None
      (Rendering|SetVisibility (Variables|Default|GetTool_04) true false))))

(fn ConstructionScript)